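; Player-controlled kart pawn that maps input axes to throttle and steering and lets the player use a held item.
; Use Item clears the held item; the first item type also sets a timed speed flag that multiplies throttle input, while the other two have no further effect.
; The E key toggles debug mode.
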(event `InputAxis|Move Forward`
  (params (AxisValue :type "Float (single-precision)"))
  (if (`self.UsingSpeedItem`)
    (`self.Set Throttle Input` (* AxisValue 1.5))
    (else
      (`self.Set Throttle Input` AxisValue))))

(event `InputAxis|Move Right`
  (params (AxisValue :type "Float (single-precision)"))
  (`self.Set Steering Input` AxisValue))

(event `Key|E`
  (params (Key :type "Key Structure"))
  (:`Pressed`
    (`self.Toggle Debug Mode`)))

(event `InputAction|Use Item`
  (params (Key :type "Key Structure"))
  (:`Pressed`
    (switch `int` (`self.Item`)
      (:`0`
        (set `self.Item` -1)
        (set `self.UsingSpeedItem` true)
        (`KismetSystemLibrary.Delay` 2.0)
        (set `self.UsingSpeedItem` false))
      (:`1`
        (set `self.Item` -1))
      (:`2`
        (set `self.Item` -1)))))

(fn `UserConstructionScript`
  (`parent.UserConstructionScript`))